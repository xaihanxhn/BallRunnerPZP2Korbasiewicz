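; BP_Crystal is a collectable crystal actor that flies into the player and disappears when touched.
; On overlap with the player pawn, it stores its current location and plays a timeline that lerps it toward the pawn's live position.
; The timeline's alpha track drives the movement, and the actor destroys itself when the timeline finishes.
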(event `self.ReceiveActorBeginOverlap`
  (params (OtherActor :type "Actor Object Reference"))
  (if (== OtherActor (`GameplayStatics.GetPlayerPawn` 0))
    (set `self.LerpStartLocation` (`self.K2_GetActorLocation`))
    (bind (_direction _smoothlepralpha) (`Timeline|TL_BlendAlpha`)
      (:`Update`
        (`self.K2_SetActorLocation` (`KismetMathLibrary.VLerp` (`self.Lerp Start Location`) (`self.K2_GetActorLocation` (`GameplayStatics.GetPlayerPawn` 0)) _smoothlepralpha)))
      (:`Finished`
        (`self.K2_DestroyActor`)))))

(fn `UserConstructionScript`)